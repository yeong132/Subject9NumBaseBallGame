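; Player controller Blueprint that connects the chat window widget and user login to the networked player state.
; On local controllers, BeginPlay waits briefly, finds the chat window and binds its message event.
; User ID is stored on BP_YMPlayerState and read back for the delayed login notification.
; Outgoing messages pass with that ID to a C++ server RPC.
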(event `self.ReceiveBeginPlay`
  ; 각 클라이언트만 UI 인스턴스 설정
  (if (`self.IsLocalPlayerController`)
    (`KismetSystemLibrary.Delay` 2.0)
    (bind _foundwidgets (`WidgetBlueprintLibrary.GetAllWidgetsOfClass` "/Game/Widgets/Widget_ChatWindow.Widget_ChatWindow_C"))
    (bind _output_get (set `self.Widget` (`|GetArrayItem` _foundwidgets)))
    ; 플레이어가 입력을 보내면 서버로 메시지 보내는 이벤트랑 Bind
    (bind _aswidget_chat_window (cast `/Game/Widgets/Widget_ChatWindow` _output_get))
    (set `self.ChatWindowWidget` _aswidget_chat_window)
    (add `/Game/Widgets/Widget_ChatWindow.SetMessageToUserController` _aswidget_chat_window (`|CreateDelegate` :!event `OnSendMsgToServer`))))

(event `SetUserId`
  (params (UserId :type String))
  ; UserId 설정은 서버RPC로 만들기
  (bind _asbp_ymplayer_state (cast `/Game/Blueprints/BP_YMPlayerState` (`self.PlayerState`)))
  (set `YMPlayerState.UserId` UserId _asbp_ymplayer_state))

(event `OnUserLoginWithId`
  ; UserId로 로그인 했을 때의 이벤트는 클라이언트 RPC로 설정
  (`KismetSystemLibrary.Delay` 2.0)
  (bind _asbp_ymplayer_state (cast `/Game/Blueprints/BP_YMPlayerState` (`self.PlayerState`)))
  (`self.OnUserLogin` (`YMPlayerState.UserId` _asbp_ymplayer_state)))

(event `OnSendMsgToServer`
  (params (Msg :type String))
  ; 블루프린트의 서버RPC랑 C++의 서버RPC랑 연결
  (set `self.Msg` Msg)
  (bind _asbp_ymplayer_state (cast `/Game/Blueprints/BP_YMPlayerState` (`self.PlayerState`)))
  (`self.Server_OnSendPlayerControllerToServer` (`self.Msg`) (`YMPlayerState.UserId` _asbp_ymplayer_state)))

(fn `UserConstructionScript`)